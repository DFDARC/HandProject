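; DoorBP is a door that swings open and closed through an Interact event.
; Interact snaps the Door component between zero and 90-degree rotation, tracking state in IsOpen, while OpenDoorT only opens it.
; BeginPlay calls EnableInput on player controller 0, passing that controller to itself.
; The Box overlap casts to BP_ThirdPersonCharacter without further effect, and OpenClose is empty, as leftover proximity-based open/close logic sits disconnected.
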(event OnComponentBeginOverlap(Door)
  (params (OverlappedComponent :type Primitive%20Component%20Object%20Reference) (OtherActor :type Actor%20Object%20Reference) (OtherComp :type Primitive%20Component%20Object%20Reference) (OtherBodyIndex :type Integer) (bFromSweep :type Boolean) (SweepResult :type Hit%20Result%20Structure%20%28by%20ref%29)))

(event OnComponentBeginOverlap(Box)
  (params (OverlappedComponent :type Primitive%20Component%20Object%20Reference) (OtherActor :type Actor%20Object%20Reference) (OtherComp :type Primitive%20Component%20Object%20Reference) (OtherBodyIndex :type Integer) (bFromSweep :type Boolean) (SweepResult :type Hit%20Result%20Structure%20%28by%20ref%29))
  (Utilities|Casting|CastToBP_ThirdPersonCharacter OtherActor)
  (if true
    _))

(event OnComponentEndOverlap(Box)
  (params (OverlappedComponent :type Primitive%20Component%20Object%20Reference) (OtherActor :type Actor%20Object%20Reference) (OtherComp :type Primitive%20Component%20Object%20Reference) (OtherBodyIndex :type Integer)))

(event Custom|OpenDoorT
  (Transformation|SetRelativeRotation (Variables|Default|GetDoor) "0.000000,90.000000,0.000000" false false))

(event EventBeginPlay
  (bind _returnvalue (Game|GetPlayerController 0))
  (Input|EnableInput _returnvalue _returnvalue))

(event Collision|EventActorBeginOverlap
  (params (OtherActor :type Actor%20Object%20Reference)))

(event EventTick
  (params (DeltaSeconds :type Float%20%28single-precision%29)))

(event EventInteract
  (if (Variables|Default|GetbIsOpen)
    (Transformation|SetRelativeRotation (Variables|Default|GetDoor) "0, 0, 0" false false)
    (Variables|Default|SetbIsOpen false)
    (else
      (Transformation|SetRelativeRotation (Variables|Default|GetDoor) "0.000000,90.000000,0.000000" false false)
      (Variables|Default|SetbIsOpen true))))

(fn ConstructionScript)

(fn OpenClose)